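; Openable door actor that swings open and closed through an OpenDoor interface.
; On begin play it stores its starting yaw, then a Door_swing timeline lerps the actor's yaw 85 degrees in the negative direction from that value.
; Closing reverses the same timeline, and a timeline event track plays the door sound at the actor's location.
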(event OnOpen(OpenDoor)
  (bind _newvar_0 (Variables|Default|GetNewVar_0))
  (bind _open_angle (Timeline|door_swing Play)
    (:Update
      (Transformation|SetActorRotation (Math|Rotator|MakeRotator 0.0 0.0 (Math|Float|Lerp _newvar_0 (+ _newvar_0 -85.0) _open_angle))))
    (:sound_timing
      (Audio|PlaySoundatLocation "/Game/Audio/door_open_1.door_open_1" (Transformation|GetActorLocation) "0, 0, 0" 1.0 1.0 0.0 0 0 0))))

(event OnClose(OpenDoor)
  (bind _newvar_0 (Variables|Default|GetNewVar_0))
  (bind _open_angle (Timeline|door_swing Reverse)
    (:Update
      (Transformation|SetActorRotation (Math|Rotator|MakeRotator 0.0 0.0 (Math|Float|Lerp _newvar_0 (+ _newvar_0 -85.0) _open_angle))))
    (:sound_timing
      (Audio|PlaySoundatLocation "/Game/Audio/door_open_1.door_open_1" (Transformation|GetActorLocation) "0, 0, 0" 1.0 1.0 0.0 0 0 0))))

(event EventBeginPlay
  (Variables|Default|SetNewVar_0 (.yaw (Transformation|GetActorRotation))))

(fn ConstructionScript)